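; Win-zone trigger actor that declares victory when the player and all three colored NPCs are inside it at once.
; Box overlap begin and end events cast the other actor to ThirdPersonCharacter, NPC_Azul, NPCRojo or NPCMorado, setting or clearing a matching presence flag.
; Each recognized entry checks all four flags and prints "GANO" when all are set.
; Victory is only a printed message, alongside a name print for every overlapping actor.
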(event `self.Box.OnComponentBeginOverlap`
  (params (OverlappedComponent :type "PrimitiveComponent Object Reference") (OtherActor :type "Actor Object Reference") (OtherComp :type "PrimitiveComponent Object Reference") (OtherBodyIndex :type Integer) (bFromSweep :type Boolean) (SweepResult :type "HitResult Structure (by ref)"))
  (`KismetSystemLibrary.PrintString` (`KismetSystemLibrary.GetDisplayName` OtherActor))
  (cast `/Game/ThirdPersonBP/Blueprints/ThirdPersonCharacter` OtherActor
    (:`then`
      (set `self.ThirdPerson` true))
    (:`CastFailed`
      (cast `/Game/ThirdPersonBP/Blueprints/NPC_Azul` OtherActor
        (:`then`
          (set `self.Azul` true))
        (:`CastFailed`
          (cast `/Game/ThirdPersonBP/Blueprints/NPCRojo` OtherActor
            (:`then`
              (set `self.Rojo` true))
            (:`CastFailed`
              (cast `/Game/ThirdPersonBP/Blueprints/NPCMorado` OtherActor)
              (set `self.Morado` true)))))))
  (if (and (`self.Azul`) (`self.Rojo`) (`self.Morado`) (`self.ThirdPerson`))
    (`KismetSystemLibrary.PrintString` "GANO")))

(event `self.Box.OnComponentEndOverlap`
  (params (OverlappedComponent :type "PrimitiveComponent Object Reference") (OtherActor :type "Actor Object Reference") (OtherComp :type "PrimitiveComponent Object Reference") (OtherBodyIndex :type Integer))
  (cast `/Game/ThirdPersonBP/Blueprints/ThirdPersonCharacter` OtherActor
    (:`then`
      (set `self.ThirdPerson` false))
    (:`CastFailed`
      (cast `/Game/ThirdPersonBP/Blueprints/NPC_Azul` OtherActor
        (:`then`
          (set `self.Azul` false))
        (:`CastFailed`
          (cast `/Game/ThirdPersonBP/Blueprints/NPCRojo` OtherActor
            (:`then`
              (set `self.Rojo` false))
            (:`CastFailed`
              (cast `/Game/ThirdPersonBP/Blueprints/NPCMorado` OtherActor)
              (set `self.Morado` false))))))))

(fn `UserConstructionScript`)